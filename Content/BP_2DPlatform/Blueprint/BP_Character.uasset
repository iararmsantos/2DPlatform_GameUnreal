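; Player character for a 2D Paper2D platformer, with walk, sprint, jump, dash, wall slide and wall jump, melee and limited axe throws.
; Tick selects flipbooks from movement state, detects walls with a forward trace, and turns the controller to face movement.
; Melee applies damage through a delayed forward line trace.
; Taking damage, or pressing debug-style key 1, costs one Health, updates the HUD and shakes the camera.
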(event Custom|UpdateAnimation
  ;[1 1 1] Handle Animation
  (if (Variables|Default|GetisDashing?)
    (Sprite|SetFlipbook (Variables|Default|GetSprite) (Variables|Animation|Getdash))
    (elif (AI|Components|NavMovement|IsFalling (Variables|Character|GetCharacterMovement))
      (Components|Capsule|SetCapsuleRadius (Variables|Collision|GetCapsuleComponent) 1.0 true)
      (if (Variables|Default|GetwallSlide?)
        (Sprite|SetFlipbook (Variables|Default|GetSprite) (Variables|Animation|GetwallSlide))
        (else
          (Sprite|SetFlipbook (Variables|Default|GetSprite) (select (< (.z (Transformation|GetVelocity)) 0.0) (Variables|Animation|Getfalling) (Variables|Animation|Getjumping)))))
      (else
        (Components|Capsule|SetCapsuleRadius (Variables|Collision|GetCapsuleComponent) 32.0 true)
        (if (Variables|Default|GetisAttacking?)
          (Sprite|SetFlipbook (Variables|Default|GetSprite) (Variables|Animation|GetattackingAnimation))
          (else
            (Sprite|SetFlipbook (Variables|Default|GetSprite) (select (> (Math|Vector|VectorLength (Transformation|GetVelocity)) 0.0) (Variables|Animation|Getrun) (Variables|Animation|Getidle)))))))))

(event Custom|WallSlideMechanic
  (bind _returnvalue (Transformation|GetActorLocation))
  (if (AI|Components|NavMovement|IsFalling (Variables|Character|GetCharacterMovement))
    (bind _outhit (Collision|LineTraceByChannel _returnvalue (+ _returnvalue (* (Transformation|GetActorForwardVector) (Math|Vector|MakeVector 5e+01 0.0 0.0))) "TraceTypeQuery1" false 0 "None"))
    (Variables|Default|SetwallSlide? (.bBlockingHit (Collision|BreakHitResult _outhit)))
    (else
      (Variables|Default|SetwallSlide? false))))

(event EventBeginPlay
  (Variables|/Script/Engine.CharacterMovementComponent|SetMaxWalkSpeed (Variables|Character|GetCharacterMovement) (Variables|Default|GetplayerSpeed))
  (bind _returnvalue (UserInterface|CreateWidget "/Game/BP_2DPlatform/Widget/WB_PlayerHUD.WB_PlayerHUD_C"))
  (bind _output_get (Variables|Components|SetplayerHUD _returnvalue))
  (UserInterface|Viewport|AddtoViewport _output_get 0))

(event Collision|EventActorBeginOverlap
  (params (OtherActor :type Actor%20Object%20Reference)))

(event EventTick
  (params (DeltaSeconds :type Float%20%28single-precision%29))
  (bind _returnvalue (Pawn|GetController))
  (bind _returnvalue_2 (Pawn|GetController))
  (CallFunction|UpdateAnimation)
  (CallFunction|WallSlideMechanic)
  (if (not (Variables|Default|GetwallSlide?))
    (Math|Float|CompareFloat (.x (Variables|/Script/Engine.MovementComponent|GetVelocity (Variables|Character|GetCharacterMovement))) 0.0
      (:>
        (Utilities|IsValid _returnvalue_2 :!label _label
          (:Is%20Valid
            (Pawn|SetControlRotation _returnvalue_2 (Math|Rotator|MakeRotator 0.0 0.0 0.0)))))
      (:==
        (if (Variables|Default|GetIsMovingRight?)
          (goto _label)
          (else
            (Utilities|IsValid _returnvalue :!label _label_2
              (:Is%20Valid
                (Pawn|SetControlRotation _returnvalue (Math|Rotator|MakeRotator 0.0 0.0 1.8e+02)))))))
      (:<
        (goto _label_2)))))

(event Game|Damage|EventAnyDamage
  (params (Damage :type Float%20%28single-precision%29) (DamageType :type Damage%20Type%20Object%20Reference) (InstigatedBy :type Controller%20Object%20Reference) (DamageCauser :type Actor%20Object%20Reference))
  (Variables|Default|Sethealth (- (Variables|Default|Gethealth) 1.0))
  (Default|UpdateHealth (Variables|Components|GetplayerHUD))
  (Camera|PlayWorldCameraShake "/Game/BP_2DPlatform/Blueprint/BP_DamagedCameraShake.BP_DamagedCameraShake_C" (Transformation|GetActorLocation) 0.0 2e+03 1.0 true))

(event Input|ActionEvents|InputActionJump
  (params (Key :type Key%20Structure :default "None"))
  ;[1 1 1] Handle Input Events
  (:Pressed
    (if (Variables|Default|GetwallSlide?)
      (Character|LaunchCharacter (Math|Vector|MakeVector (* (.x (Transformation|GetActorForwardVector)) -1.5e+03) 0.0 6.5e+02) true true)
      (else
        (Character|Jump))))
  (:Released
    (Character|StopJumping)))

(event Input|ActionEvents|InputActionSprint
  (params (Key :type Key%20Structure :default "None"))
  ;[1 1 1] Handle Input Events
  (:Pressed
    (Variables|/Script/Engine.CharacterMovementComponent|SetMaxWalkSpeed (Variables|Character|GetCharacterMovement) (Variables|Default|GetsprintSpeed)))
  (:Released
    (Variables|/Script/Engine.CharacterMovementComponent|SetMaxWalkSpeed (Variables|Character|GetCharacterMovement) (Variables|Default|GetplayerSpeed))))

(event Input|ActionEvents|InputActionDash
  (params (Key :type Key%20Structure :default "None"))
  ;[1 1 1] Handle Input Events
  (:Pressed
    (Character|LaunchCharacter (Math|Vector|MakeVector (select (Variables|Default|GetIsMovingRight?) 3.3e+03 -3.3e+03) 0.0 0.0) true false)
    (Variables|Default|SetisDashing? true)
    (Utilities|FlowControl|RetriggerableDelay (Class|PaperFlipbook|GetTotalDuration (Variables|Animation|Getdash)))
    (Variables|Default|SetisDashing? false)))

(event Input|ActionEvents|InputActionMeleeAttack
  (params (Key :type Key%20Structure :default "None"))
  (bind _returnvalue (Transformation|GetActorLocation))
  (:Pressed
    (if (not (or (Variables|Default|GetwallSlide?) (AI|Components|NavMovement|IsFalling (Variables|Character|GetCharacterMovement))))
      (Variables|Default|SetisAttacking? true)
      (Development|PrintString (Utilities|String|ToString(Float) (Class|PaperFlipbook|GetTotalDuration (Variables|Animation|GetattackingAnimation))))
      (Utilities|FlowControl|Delay 0.5)
      (Utilities|FlowControl|Sequence
        (:then_0
          (Variables|Default|SetisAttacking? false))
        (:then_1
          (bind _outhit (Collision|LineTraceForObjects _returnvalue (+ _returnvalue (* (Transformation|GetActorForwardVector) "100.000000,0,0")) (Utilities|Array|MakeArray "ObjectTypeQuery3") false (Utilities|Array|MakeArray self) "ForDuration"))
          (Development|PrintString (Utilities|GetDisplayName (.HitActor (Collision|BreakHitResult _outhit))))
          (Game|Damage|ApplyDamage (.HitActor (Collision|BreakHitResult _outhit)) 1.0 0 0))))))

(event Input|ActionEvents|InputActionProjectileAttack
  (params (Key :type Key%20Structure :default "None"))
  (:Pressed
    (if (> (Variables|Default|GetnumberOfAxes) 0.0)
      (Game|SpawnActorfromClass "/Game/BP_2DPlatform/Blueprint/BP_Axe.BP_Axe_C" (Math|Transform|MakeTransform (Transformation|GetWorldLocation (Variables|Default|GetAxeSpawn)) (select (Variables|Default|GetIsMovingRight?) "0, 0, 0" "-180.000000, 0, 0") "1.000000,1.000000,1.000000") "Undefined" 0 0)
      (Variables|Default|SetnumberOfAxes (- (Variables|Default|GetnumberOfAxes) 1.0)))))

(event Input|AxisEvents|InputAxisMoveRight
  (params (AxisValue :type Float%20%28single-precision%29))
  ;[1 1 1] Handle Input Events
  (if (> AxisValue 0.0)
    (Variables|Default|SetIsMovingRight? true)
    (elif (< AxisValue 0.0)
      (Variables|Default|SetIsMovingRight? false)))
  (Pawn|Input|AddMovementInput "1.000000, 0, 0" AxisValue false))

(event Input|KeyboardEvents|1
  (params (Key :type Key%20Structure :default "None"))
  (:Pressed
    (Variables|Default|Sethealth (- (Variables|Default|Gethealth) 1.0))
    (Default|UpdateHealth (Variables|Components|GetplayerHUD))
    (Camera|PlayWorldCameraShake "/Game/BP_2DPlatform/Blueprint/BP_DamagedCameraShake.BP_DamagedCameraShake_C" (Transformation|GetActorLocation) 0.0 2e+03 1.0 true)))

(fn ConstructionScript
  (Variables|Default|SetheartContainers (Math|Float|Truncate (Variables|Default|Gethealth))))