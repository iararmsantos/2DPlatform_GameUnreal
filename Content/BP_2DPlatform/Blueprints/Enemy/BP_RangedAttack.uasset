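; Ranged enemy character for a 2D platformer that faces the player, shoots projectiles and drops a coin on death.
; Flipbooks and health load from a data table row matching EnemyType, and Tick picks the flipbook by state.
; Player overlap with AttackBox starts a looping timer, never cleared here, firing animation-timed shots gated by a cooldown.
; Damage knocks it back, while falling-player stomps bounce the player and share the hurt/death logic.
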(event OnComponentBeginOverlap(Box)
  (params (OverlappedComponent :type Primitive%20Component%20Object%20Reference) (OtherActor :type Actor%20Object%20Reference) (OtherComp :type Primitive%20Component%20Object%20Reference) (OtherBodyIndex :type Integer) (bFromSweep :type Boolean) (SweepResult :type Hit%20Result%20Structure%20%28by%20ref%29))
  ;[1 1 1] Receiving Damage by Jump
  (bind _asbp_character (Utilities|Casting|CastToBP_Character OtherActor))
  (if (AI|Components|NavMovement|IsFalling (Variables|/Script/Engine.Character|GetCharacterMovement _asbp_character))
    (Variables|Default|SetenemyHealth (- (Variables|Default|GetenemyHealth) (Variables|/Game/BP_2DPlatform/Blueprints/Character/BP_Character.BP_Character_C|GetjumpDamage _asbp_character)))
    (CallFunction|JumpDamage)
    (Character|LaunchCharacter _asbp_character "0, 0,500.000000" true true)))

(event OnComponentBeginOverlap(attackBox)
  (params (OverlappedComponent :type Primitive%20Component%20Object%20Reference) (OtherActor :type Actor%20Object%20Reference) (OtherComp :type Primitive%20Component%20Object%20Reference) (OtherBodyIndex :type Integer) (bFromSweep :type Boolean) (SweepResult :type Hit%20Result%20Structure%20%28by%20ref%29))
  ;[1 1 1] Enemy attacking by Range
  (Utilities|Casting|CastToBP_Character OtherActor)
  (bind _returnvalue (Utilities|Time|SetTimerbyEvent (delegate Custom|Attack%20Player) 1.0 true))
  (Variables|Default|SetattackEvent _returnvalue))

(event Custom|Handle%20Animation
  ;[1 1 1] Changing Animation
  (if (Variables|Default|GetenemyDead?)
    (Sprite|SetFlipbook (Variables|Default|GetSprite) (select (Variables|Default|GetenemyDeadBody?) (Variables|Default|GetEnemyDeadBody) (Variables|Default|GetEnemyDied)))
    (elif (Variables|Default|GetenemyDamaged?)
      (Sprite|SetFlipbook (Variables|Default|GetSprite) (Variables|Default|GetEnemyDamaged))
      (elif (Variables|Default|GetisRangedAttack?)
        (Sprite|SetFlipbook (Variables|Default|GetSprite) (Variables|Default|GetEnemyRangedAttack))
        (else
          (Sprite|SetFlipbook (Variables|Default|GetSprite) (select (> (Math|Vector|VectorLength (Variables|/Script/Engine.MovementComponent|GetVelocity (Variables|Character|GetCharacterMovement))) 0.0) (Variables|Default|GetEnemyMoving) (Variables|Default|GetEnemyIdle))))))))

(event Custom|Handle%20Rotation
  ;[1 1 1] Handling Rotation
  (if (not (Variables|Default|GetenemyDead?))
    (if (< (.x (Math|Vector|Normalize (Math|Vector|GetUnitDirection(Vector) (Transformation|GetActorLocation (Game|GetPlayerCharacter 0)) (Transformation|GetActorLocation)))) 0.0)
      (Transformation|SetActorRotation "0, 0, 0")
      (else
        (Transformation|SetActorRotation "0,180.000000, 0")))))

(event Custom|Jump%20Damage
  ;[1 1 1] Receiving Damage
  (if (<= (Variables|Default|GetenemyHealth) 0.0)
    (Utilities|FlowControl|DoOnce false
      (:Completed
        (Components|DestroyComponent (Variables|Default|GetBox))
        (Variables|Default|SetenemyDead? true)
        (Utilities|FlowControl|Delay (- (Class|PaperFlipbook|GetTotalDuration (Variables|Default|GetEnemyDied)) 0.4))
        (Variables|Default|SetenemyDeadBody? true)
        (Collision|SetCollisionProfileName (Variables|Collision|GetCapsuleComponent) "OverlapOnlyPawn" true :!class /Script/Engine.PrimitiveComponent)
        (Game|SpawnActorfromClass "/Game/BP_2DPlatform/Blueprints/Collectibles/BP_enemyCoin.BP_enemyCoin_C" (Math|Transform|MakeTransform (Transformation|GetActorLocation) "0, 0, 0" "1.000000,1.000000,1.000000") "Undefined" 0 (Math|Conversions|ToFloat(Integer) (Math|Float|Round (Math|Random|RandomFloatinRange 1.0 1e+01))) 0)))
    (else
      (Variables|Default|SetenemyDamaged? true)
      (Audio|PlaySound2D "/Game/SoundEffects/Sword_Hit_+_Slash/Hurt.Hurt" 1.0 1.0 0.0 0 0)
      (Utilities|FlowControl|RetriggerableDelay (Class|PaperFlipbook|GetTotalDuration (Variables|Default|GetEnemyDamaged)))
      (Variables|Default|SetenemyDamaged? false))))

(event Custom|Attack%20Player
  ;[1 1 1] Enemy attacking by Range
  (if (not (Variables|Default|GetenemyDead?))
    (Utilities|FlowControl|DoOnce false :!label _label
      (:Completed
        (Variables|Default|SetisRangedAttack? true)
        (Utilities|FlowControl|Delay (Class|PaperFlipbook|GetTotalDuration (Variables|Default|GetEnemyRangedAttack)))
        (if (not (Variables|Default|GetenemyDead?))
          (Game|SpawnActorfromClass (Variables|Default|GetenemyProjectile) (Math|Transform|MakeTransform (Transformation|GetWorldLocation (Variables|Default|GetProjectileSpawnLocation)) (Transformation|GetActorRotation) "1.000000,1.000000,1.000000") "Undefined" 0 0)
          (Variables|Default|SetisRangedAttack? false)
          (Utilities|FlowControl|Delay (Variables|Default|GetcoolDown))
          (goto _label Reset))))))

(event EventBeginPlay
  ;[1 1 1] Changing Sprites
  (Variables|/Script/Engine.CharacterMovementComponent|SetMaxWalkSpeed (Variables|Character|GetCharacterMovement) (Variables|Default|GetenemyWalkSpeed))
  (bind _outrownames (DataTable|GetDataTableRowNames "/Game/Sprites/Enemies/EnemyDataTable.EnemyDataTable"))
  (for _array_element _outrownames
    (bind _returnvalue (Utilities|GetDataTableRow "/Game/Sprites/Enemies/EnemyDataTable.EnemyDataTable" _array_element)
      (:then
        (if (Utilities|Enum|Equal(Enum) (Variables|Default|GetenemyType) (.enemytype _returnvalue))
          (Variables|Default|SetEnemyIdle (.idle _returnvalue))
          (Variables|Default|SetEnemyMoving (.moving _returnvalue))
          (Variables|Default|SetEnemyAttacking (.attacking _returnvalue))
          (Variables|Default|SetEnemyRangedAttack (.rangedattack _returnvalue))
          (Variables|Default|SetEnemyDamaged (.damaged _returnvalue))
          (Variables|Default|SetEnemyDied (.died _returnvalue))
          (Variables|Default|SetEnemyDeadBody (.deathbody _returnvalue))
          (Variables|Default|SetenemyHealth (.enemyhealth _returnvalue)))))))

(event EventTick
  (params (DeltaSeconds :type Float%20%28single-precision%29))
  ;[1 1 1] Starting Animation and Movement
  (CallFunction|HandleAnimation)
  (CallFunction|HandleRotation))

(event Game|Damage|EventAnyDamage
  (params (Damage :type Float%20%28single-precision%29) (DamageType :type Damage%20Type%20Object%20Reference) (InstigatedBy :type Controller%20Object%20Reference) (DamageCauser :type Actor%20Object%20Reference))
  ;[1 1 1] Receiving Damage
  (Variables|Default|SetenemyHealth (- (Variables|Default|GetenemyHealth) Damage))
  (Character|LaunchCharacter (Math|Vector|MakeVector (* (select (< (.x (Math|Vector|Normalize (Math|Vector|GetUnitDirection(Vector) (Transformation|GetActorLocation DamageCauser) (Transformation|GetActorLocation)))) 0.0) 1.0 -1.0) -1.5e+03) 0.0 0.0) true true)
  (if (<= (Variables|Default|GetenemyHealth) 0.0)
    (Utilities|FlowControl|DoOnce false
      (:Completed
        (Components|DestroyComponent (Variables|Default|GetBox))
        (Variables|Default|SetenemyDead? true)
        (Utilities|FlowControl|Delay (- (Class|PaperFlipbook|GetTotalDuration (Variables|Default|GetEnemyDied)) 0.4))
        (Variables|Default|SetenemyDeadBody? true)
        (Collision|SetCollisionProfileName (Variables|Collision|GetCapsuleComponent) "OverlapOnlyPawn" true :!class /Script/Engine.PrimitiveComponent)
        (Game|SpawnActorfromClass "/Game/BP_2DPlatform/Blueprints/Collectibles/BP_enemyCoin.BP_enemyCoin_C" (Math|Transform|MakeTransform (Transformation|GetActorLocation) "0, 0, 0" "1.000000,1.000000,1.000000") "Undefined" 0 (Math|Conversions|ToFloat(Integer) (Math|Float|Round (Math|Random|RandomFloatinRange 1.0 1e+01))) 0)))
    (else
      (Variables|Default|SetenemyDamaged? true)
      (Audio|PlaySound2D "/Game/SoundEffects/Sword_Hit_+_Slash/Hurt.Hurt" 1.0 1.0 0.0 0 0)
      (Utilities|FlowControl|RetriggerableDelay (Class|PaperFlipbook|GetTotalDuration (Variables|Default|GetEnemyDamaged)))
      (Variables|Default|SetenemyDamaged? false))))

(fn ConstructionScript
  (bind _outrownames (DataTable|GetDataTableRowNames "/Game/Sprites/Enemies/EnemyDataTable.EnemyDataTable"))
  (for _array_element _outrownames
    (bind _returnvalue (Utilities|GetDataTableRow "/Game/Sprites/Enemies/EnemyDataTable.EnemyDataTable" _array_element)
      (:then
        (if (Utilities|Enum|Equal(Enum) (Variables|Default|GetenemyType) (.enemytype _returnvalue))
          (Variables|Default|SetEnemyIdle (.idle _returnvalue))
          (Variables|Default|SetEnemyMoving (.moving _returnvalue))
          (Variables|Default|SetEnemyAttacking (.attacking _returnvalue))
          (Variables|Default|SetEnemyRangedAttack (.rangedattack _returnvalue))
          (Variables|Default|SetEnemyDamaged (.damaged _returnvalue))
          (Variables|Default|SetEnemyDied 0)
          (Variables|Default|SetEnemyDied (.died _returnvalue))
          (Variables|Default|SetEnemyDeadBody (.deathbody _returnvalue))
          (Variables|Default|SetenemyHealth (.enemyhealth _returnvalue))
          (Sprite|SetFlipbook (Variables|Default|GetSprite) (Variables|Default|GetEnemyIdle)))))))