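; 2D platformer enemy that patrols, attacks the player and drops a coin on death.
; Flipbooks and health come from a data table row matched by enemy type, and Tick selects the animation and drives movement.
; Line traces turn it around at walls and ledges after a pause.
; An attack-box timer triggers short forward-trace hits with a cooldown, while damage knocks it back and falling players can stomp it and bounce off.
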(event OnComponentBeginOverlap(Box)
  (params (OverlappedComponent :type Primitive%20Component%20Object%20Reference) (OtherActor :type Actor%20Object%20Reference) (OtherComp :type Primitive%20Component%20Object%20Reference) (OtherBodyIndex :type Integer) (bFromSweep :type Boolean) (SweepResult :type Hit%20Result%20Structure%20%28by%20ref%29))
  ;[1 1 1] Receiving Damage by Jump
  (bind _asbp_character (Utilities|Casting|CastToBP_Character OtherActor))
  (if (AI|Components|NavMovement|IsFalling (Variables|/Script/Engine.Character|GetCharacterMovement _asbp_character))
    (Variables|Default|SetenemyHealth (- (Variables|Default|GetenemyHealth) (Variables|/Game/BP_2DPlatform/Blueprints/Character/BP_Character.BP_Character_C|GetjumpDamage _asbp_character)))
    (CallFunction|JumpDamage)
    (Character|LaunchCharacter _asbp_character "0, 0,500.000000" true true)))

(event OnComponentBeginOverlap(attackBox)
  (params (OverlappedComponent :type Primitive%20Component%20Object%20Reference) (OtherActor :type Actor%20Object%20Reference) (OtherComp :type Primitive%20Component%20Object%20Reference) (OtherBodyIndex :type Integer) (bFromSweep :type Boolean) (SweepResult :type Hit%20Result%20Structure%20%28by%20ref%29))
  ;[1 1 1] Enemy attacking by Range
  (Utilities|Casting|CastToBP_Character OtherActor)
  (bind _returnvalue (Utilities|Time|SetTimerbyEvent (delegate Custom|Attack%20Player) 1.0 true))
  (Variables|Default|SetattackEvent _returnvalue))

(event OnComponentEndOverlap(attackBox)
  (params (OverlappedComponent :type Primitive%20Component%20Object%20Reference) (OtherActor :type Actor%20Object%20Reference) (OtherComp :type Primitive%20Component%20Object%20Reference) (OtherBodyIndex :type Integer))
  (bind _returnvalue (Transformation|GetActorLocation))
  ;[1 1 1] Finishing enemy Atacking
  (Utilities|Casting|CastToBP_Character OtherActor)
  (Utilities|Time|ClearandInvalidateTimerbyHandle (Variables|Default|GetattackEvent))
  ;[1 1 1] Enemy attacking by Range
  (Utilities|FlowControl|DoOnce false) ; enters at Reset
)

(event Custom|Handle%20Animation
  ;[1 1 1] Changing Animation
  (if (Variables|Default|GetenemyDead?)
    (Sprite|SetFlipbook (Variables|Default|GetSprite) (select (Variables|Default|GetenemyDeadBody?) (Variables|Default|GetEnemyDeadBody) (Variables|Default|GetEnemyDied)))
    (elif (Variables|Default|GetenemyDamaged?)
      (Sprite|SetFlipbook (Variables|Default|GetSprite) (Variables|Default|GetEnemyDamaged))
      (elif (Variables|Default|GetisAttacking?)
        (Sprite|SetFlipbook (Variables|Default|GetSprite) (Variables|Default|GetEnemyAttacking))
        (else
          (Sprite|SetFlipbook (Variables|Default|GetSprite) (select (> (Math|Vector|VectorLength (Variables|/Script/Engine.MovementComponent|GetVelocity (Variables|Character|GetCharacterMovement))) 0.0) (Variables|Default|GetEnemyMoving) (Variables|Default|GetEnemyIdle))))))))

(event Custom|Handle%20Movement
  (bind _returnvalue (Transformation|GetActorLocation))
  (bind _returnvalue_2 (Transformation|GetActorLocation))
  ;[1 1 1] Moving Character
  (if (not (Variables|Default|GetenemyDead?))
    (Utilities|FlowControl|Sequence
      (:then_0
        (if (Variables|Default|GetenemyDamaged?)
          (if (> (Variables|Default|GethitDirection) 0.0)
            (Transformation|SetActorRotation "0, 0, 0")
            (else
              (Transformation|SetActorRotation "0,180.000000, 0")))
          (elif (> (Variables|Default|GetmovementDirection) 0.0)
            (Transformation|SetActorRotation "0, 0, 0")
            (else
              (Transformation|SetActorRotation "0,180.000000, 0")))))
      (:then_1
        (if (Variables|Default|GetcanMove?)
          (if (not (or (Variables|Default|GetenemyDamaged?) (Variables|Default|GetisAttacking?)))
            (Pawn|Input|AddMovementInput "1.000000, 0, 0" (Variables|Default|GetmovementDirection) false)
            (Utilities|FlowControl|Sequence
              (:then_0
                (bind _returnvalue_3 (Collision|LineTraceByChannel _returnvalue (+ _returnvalue (* (Transformation|GetActorForwardVector) (Math|Vector|MakeVector 5e+01 0.0 0.0))) "TraceTypeQuery1" false 0 "None"))
                (if _returnvalue_3
                  (Utilities|FlowControl|DoOnce false :!label _label
                    (:Completed
                      (Variables|/Script/Engine.CharacterMovementComponent|SetMaxWalkSpeed (Variables|Character|GetCharacterMovement) 0.0)
                      (Utilities|FlowControl|Delay (Variables|Default|GetwaitTime))
                      (Variables|/Script/Engine.CharacterMovementComponent|SetMaxWalkSpeed (Variables|Character|GetCharacterMovement) (Variables|Default|GetenemyWalkSpeed))
                      (Variables|Default|SetmovementDirection (* (Variables|Default|GetmovementDirection) -1.0))
                      (goto _label Reset)))))
              (:then_1
                (bind _returnvalue_4 (Collision|LineTraceByChannel _returnvalue_2 (+ (- _returnvalue_2 "0,0,100.000000") (* (Transformation|GetActorForwardVector) (Math|Vector|MakeVector 1e+02 0.0 0.0))) "TraceTypeQuery1" false 0 "None"))
                (if (not _returnvalue_4)
                  (goto _label))))))))))

(event Custom|Jump%20Damage
  ;[1 1 1] Receiving Damage
  (if (<= (Variables|Default|GetenemyHealth) 0.0)
    (Utilities|FlowControl|DoOnce false
      (:Completed
        (Components|DestroyComponent (Variables|Default|GetBox))
        (Variables|Default|SetenemyDead? true)
        (Utilities|FlowControl|Delay (- (Class|PaperFlipbook|GetTotalDuration (Variables|Default|GetEnemyDied)) 0.4))
        (Variables|Default|SetenemyDeadBody? true)
        (Collision|SetCollisionProfileName (Variables|Collision|GetCapsuleComponent) "OverlapOnlyPawn" true :!class /Script/Engine.PrimitiveComponent)
        (Game|SpawnActorfromClass "/Game/BP_2DPlatform/Blueprints/Collectibles/BP_enemyCoin.BP_enemyCoin_C" (Math|Transform|MakeTransform (Transformation|GetActorLocation) "0, 0, 0" "1.000000,1.000000,1.000000") "Undefined" 0 (Math|Conversions|ToFloat(Integer) (Math|Float|Round (Math|Random|RandomFloatinRange 1.0 1e+01))) 0)))
    (else
      (Variables|Default|SetenemyDamaged? true)
      (Utilities|FlowControl|RetriggerableDelay (Class|PaperFlipbook|GetTotalDuration (Variables|Default|GetEnemyDamaged)))
      (Variables|Default|SetenemyDamaged? false))))

(event Custom|Attack%20Player
  (bind _returnvalue (Transformation|GetActorLocation))
  ;[1 1 1] Enemy attacking by Range
  (if (not (Variables|Default|GetenemyDead?))
    (Utilities|FlowControl|DoOnce false :!label _label
      (:Completed
        (Variables|Default|SetisAttacking? true)
        (Utilities|FlowControl|Delay (Class|PaperFlipbook|GetTotalDuration (Variables|Default|GetEnemyAttacking)))
        (Utilities|FlowControl|Sequence
          (:then_0
            (Variables|Default|SetisAttacking? false))
          (:then_1
            (if (not (Variables|Default|GetenemyDead?))
              (bind _outhit (Collision|LineTraceForObjects _returnvalue (+ _returnvalue (* (Transformation|GetActorForwardVector) (Math|Vector|MakeVector 1e+02 0.0 0.0))) (Utilities|Array|MakeArray "ObjectTypeQuery3") false (Utilities|Array|MakeArray self) "None"))
              (if (== (Game|GetPlayerCharacter 0) (.HitActor (Collision|BreakHitResult _outhit)))
                (Game|Damage|ApplyDamage (.HitActor (Collision|BreakHitResult _outhit)) (Variables|Default|GetenemyDamage) 0 0))
              (Utilities|FlowControl|Delay (Variables|Default|GetcoolDown))
              (goto _label Reset))))))))

(event EventBeginPlay
  ;[1 1 1] Changing Sprites
  (Variables|/Script/Engine.CharacterMovementComponent|SetMaxWalkSpeed (Variables|Character|GetCharacterMovement) (Variables|Default|GetenemyWalkSpeed))
  (bind _outrownames (DataTable|GetDataTableRowNames "/Game/Sprites/Enemies/EnemyDataTable.EnemyDataTable"))
  (for _array_element _outrownames
    (bind _returnvalue (Utilities|GetDataTableRow "/Game/Sprites/Enemies/EnemyDataTable.EnemyDataTable" _array_element)
      (:then
        (if (Utilities|Enum|Equal(Enum) (Variables|Default|GetenemyType) (.enemytype _returnvalue))
          (Variables|Default|SetEnemyIdle (.idle _returnvalue))
          (Variables|Default|SetEnemyMoving (.moving _returnvalue))
          (Variables|Default|SetEnemyAttacking (.attacking _returnvalue))
          (Variables|Default|SetEnemyRangedAttack (.rangedattack _returnvalue))
          (Variables|Default|SetEnemyDamaged (.damaged _returnvalue))
          (Variables|Default|SetEnemyDied (.died _returnvalue))
          (Variables|Default|SetEnemyDeadBody (.deathbody _returnvalue))
          (Variables|Default|SetenemyHealth (.enemyhealth _returnvalue)))))))

(event EventTick
  (params (DeltaSeconds :type Float%20%28single-precision%29))
  ;[1 1 1] Starting Animation and Movement
  (CallFunction|HandleAnimation)
  (CallFunction|HandleMovement))

(event Game|Damage|EventAnyDamage
  (params (Damage :type Float%20%28single-precision%29) (DamageType :type Damage%20Type%20Object%20Reference) (InstigatedBy :type Controller%20Object%20Reference) (DamageCauser :type Actor%20Object%20Reference))
  (bind _returnvalue (Transformation|GetActorLocation DamageCauser))
  (bind _returnvalue_2 (Transformation|GetActorLocation))
  (bind _returnvalue_3 (Math|Vector|GetUnitDirection(Vector) _returnvalue _returnvalue_2))
  (bind _returnvalue_4 (Math|Vector|Normalize _returnvalue_3))
  (bind _returnvalue_5 (< (.x _returnvalue_4) 0.0))
  (bind _returnvalue_6 (select _returnvalue_5 1.0 -1.0))
  ;[1 1 1] Receiving Damage
  (Variables|Default|SetenemyHealth (- (Variables|Default|GetenemyHealth) Damage))
  (Variables|Default|SethitDirection _returnvalue_6)
  (Character|LaunchCharacter (Math|Vector|MakeVector (* _returnvalue_6 -1.5e+03) 0.0 0.0) true true)
  (if (<= (Variables|Default|GetenemyHealth) 0.0)
    (Utilities|FlowControl|DoOnce false
      (:Completed
        (Components|DestroyComponent (Variables|Default|GetBox))
        (Variables|Default|SetenemyDead? true)
        (Utilities|FlowControl|Delay (- (Class|PaperFlipbook|GetTotalDuration (Variables|Default|GetEnemyDied)) 0.4))
        (Variables|Default|SetenemyDeadBody? true)
        (Collision|SetCollisionProfileName (Variables|Collision|GetCapsuleComponent) "OverlapOnlyPawn" true :!class /Script/Engine.PrimitiveComponent)
        (Game|SpawnActorfromClass "/Game/BP_2DPlatform/Blueprints/Collectibles/BP_enemyCoin.BP_enemyCoin_C" (Math|Transform|MakeTransform (Transformation|GetActorLocation) "0, 0, 0" "1.000000,1.000000,1.000000") "Undefined" 0 (Math|Conversions|ToFloat(Integer) (Math|Float|Round (Math|Random|RandomFloatinRange 1.0 1e+01))) 0)))
    (else
      (Variables|Default|SetenemyDamaged? true)
      (Utilities|FlowControl|RetriggerableDelay (Class|PaperFlipbook|GetTotalDuration (Variables|Default|GetEnemyDamaged)))
      (Variables|Default|SetenemyDamaged? false))))

(fn ConstructionScript
  (bind _outrownames (DataTable|GetDataTableRowNames "/Game/Sprites/Enemies/EnemyDataTable.EnemyDataTable"))
  (for _array_element _outrownames
    (bind _returnvalue (Utilities|GetDataTableRow "/Game/Sprites/Enemies/EnemyDataTable.EnemyDataTable" _array_element)
      (:then
        (if (Utilities|Enum|Equal(Enum) "NewEnumerator0" (.enemytype _returnvalue))
          (Variables|Default|SetEnemyIdle (.idle _returnvalue))
          (Variables|Default|SetEnemyMoving (.moving _returnvalue))
          (Variables|Default|SetEnemyAttacking (.attacking _returnvalue))
          (Variables|Default|SetEnemyRangedAttack (.rangedattack _returnvalue))
          (Variables|Default|SetEnemyDamaged (.damaged _returnvalue))
          (Variables|Default|SetEnemyDied (.died _returnvalue))
          (Variables|Default|SetEnemyDeadBody (.deathbody _returnvalue))
          (Variables|Default|SetenemyHealth (.enemyhealth _returnvalue))
          (Sprite|SetFlipbook (Variables|Default|GetSprite) (Variables|Default|GetEnemyIdle)))))))