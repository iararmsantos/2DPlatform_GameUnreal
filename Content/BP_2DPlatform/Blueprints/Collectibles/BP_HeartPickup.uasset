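; BP_HeartPickup is a 2D platformer collectible that restores health to the player character.
; When BP_Character overlaps its Box, a DoOnce gate adds NoHealth to the character's Health, clamped between one and MaxHealth.
; It then passes the truncated NoHealth to ShowHeart on the player's HUD, plays a 2D pickup sound and destroys itself.
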(event OnComponentBeginOverlap(Box)
  (params (OverlappedComponent :type Primitive%20Component%20Object%20Reference) (OtherActor :type Actor%20Object%20Reference) (OtherComp :type Primitive%20Component%20Object%20Reference) (OtherBodyIndex :type Integer) (bFromSweep :type Boolean) (SweepResult :type Hit%20Result%20Structure%20%28by%20ref%29))
  (bind _asbp_character (Utilities|Casting|CastToBP_Character OtherActor))
  (Utilities|FlowControl|DoOnce false
    (:Completed
      (Variables|/Game/BP_2DPlatform/Blueprints/Character/BP_Character.BP_Character_C|Sethealth _asbp_character (Math|Float|Clamp(Float) (+ (Variables|/Game/BP_2DPlatform/Blueprints/Character/BP_Character.BP_Character_C|Gethealth _asbp_character) (Variables|Default|GetnoHealth)) 1.0 (Variables|/Game/BP_2DPlatform/Blueprints/Character/BP_Character.BP_Character_C|GetmaxHealth _asbp_character)))
      (Default|ShowHeart (Variables|/Game/BP_2DPlatform/Blueprints/Character/BP_Character.BP_Character_C|GetplayerHUD _asbp_character) (Math|Float|Truncate (Variables|Default|GetnoHealth)))
      (Audio|PlaySound2D "/Game/SoundEffects/Health/Healthpickup.Healthpickup" 1.0 1.0 0.0 0 0)
      (Actor|DestroyActor))))

(event EventBeginPlay)

(event Collision|EventActorBeginOverlap
  (params (OtherActor :type Actor%20Object%20Reference)))

(event EventTick
  (params (DeltaSeconds :type Float%20%28single-precision%29)))

(fn ConstructionScript)