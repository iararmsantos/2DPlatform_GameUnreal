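; A collectible axe pickup for the 2D platformer that adds axes to the player's inventory.
; When BP_Character overlaps its Box, it adds its axe amount to the character's count, clamped to the character's maximum.
; It then writes the new count to the character's save object, saves it to a slot, plays a pickup sound and destroys itself.
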(event OnComponentBeginOverlap(Box)
  (params (OverlappedComponent :type Primitive%20Component%20Object%20Reference) (OtherActor :type Actor%20Object%20Reference) (OtherComp :type Primitive%20Component%20Object%20Reference) (OtherBodyIndex :type Integer) (bFromSweep :type Boolean) (SweepResult :type Hit%20Result%20Structure%20%28by%20ref%29))
  (bind _asbp_character (Utilities|Casting|CastToBP_Character OtherActor))
  (bind _output_get (Variables|/Game/BP_2DPlatform/Blueprints/Character/BP_Character.BP_Character_C|SetnumberOfAxes _asbp_character (Math|Float|Clamp(Float) (+ (Variables|Default|GetnoOfAxes) (Variables|/Game/BP_2DPlatform/Blueprints/Character/BP_Character.BP_Character_C|GetnumberOfAxes _asbp_character)) 0.0 (Variables|/Game/BP_2DPlatform/Blueprints/Character/BP_Character.BP_Character_C|GetmaxAxes _asbp_character))))
  (Variables|/Game/Levels/BP_SaveGame.BP_SaveGame_C|SetnumOfAxes (Variables|/Game/BP_2DPlatform/Blueprints/Character/BP_Character.BP_Character_C|GetsaveGame _asbp_character) _output_get)
  (SaveGame|SaveGametoSlot (Variables|/Game/BP_2DPlatform/Blueprints/Character/BP_Character.BP_Character_C|GetsaveGame _asbp_character) "1")
  (Audio|PlaySound2D "/Game/SoundEffects/Axe/Pickupaxe.Pickupaxe" 1.0 1.0 0.0 0 0)
  (Actor|DestroyActor))

(event EventBeginPlay)

(event Collision|EventActorBeginOverlap
  (params (OtherActor :type Actor%20Object%20Reference)))

(event EventTick
  (params (DeltaSeconds :type Float%20%28single-precision%29)))

(fn ConstructionScript)