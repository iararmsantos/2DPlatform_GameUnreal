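; Player character for a 2D side-scrolling platformer, with run, sprint, jump, dash, wall slide and wall jump.
; Tick selects the Paper2D flipbook from movement state, shrinking the capsule radius while airborne, and yaws the controller to face travel direction except during wall slides.
; A debug-drawn forward line trace while falling flags wall slides, turning Jump into a launch away from the wall.
; Dash launches horizontally, holding its flipbook for one playthrough.
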(event Custom|UpdateAnimation
  ;[1 1 1] Handle Animation
  (if (Variables|Default|GetisDashing?)
    (Sprite|SetFlipbook (Variables|Default|GetSprite) (Variables|Animation|Getdash))
    (elif (AI|Components|NavMovement|IsFalling (Variables|Character|GetCharacterMovement))
      (Components|Capsule|SetCapsuleRadius (Variables|Collision|GetCapsuleComponent) 1.0 true)
      (if (Variables|Default|GetwallSlide?)
        (Sprite|SetFlipbook (Variables|Default|GetSprite) (Variables|Animation|GetwallSlide))
        (else
          (Sprite|SetFlipbook (Variables|Default|GetSprite) (select (< (.z (Transformation|GetVelocity)) 0.0) (Variables|Animation|Getfalling) (Variables|Animation|Getjumping)))))
      (else
        (Components|Capsule|SetCapsuleRadius (Variables|Collision|GetCapsuleComponent) 32.0 true)
        (Sprite|SetFlipbook (Variables|Default|GetSprite) (select (> (Math|Vector|VectorLength (Transformation|GetVelocity)) 0.0) (Variables|Animation|Getrun) (Variables|Animation|Getidle)))))))

(event Custom|WallSlideMechanic
  (bind _returnvalue (Transformation|GetActorLocation))
  (if (AI|Components|NavMovement|IsFalling (Variables|Character|GetCharacterMovement))
    (bind _outhit (Collision|LineTraceByChannel _returnvalue (+ _returnvalue (* (Transformation|GetActorForwardVector) (Math|Vector|MakeVector 5e+01 0.0 0.0))) "TraceTypeQuery1" false 0 "ForDuration"))
    (Variables|Default|SetwallSlide? (.bBlockingHit (Collision|BreakHitResult _outhit)))
    (else
      (Variables|Default|SetwallSlide? false))))

(event EventBeginPlay
  (Variables|/Script/Engine.CharacterMovementComponent|SetMaxWalkSpeed (Variables|Character|GetCharacterMovement) (Variables|Default|GetplayerSpeed)))

(event Collision|EventActorBeginOverlap
  (params (OtherActor :type Actor%20Object%20Reference)))

(event EventTick
  (params (DeltaSeconds :type Float%20%28single-precision%29))
  (bind _returnvalue (Pawn|GetController))
  (bind _returnvalue_2 (Pawn|GetController))
  (CallFunction|UpdateAnimation)
  (CallFunction|WallSlideMechanic)
  (if (not (Variables|Default|GetwallSlide?))
    (Math|Float|CompareFloat (.x (Variables|/Script/Engine.MovementComponent|GetVelocity (Variables|Character|GetCharacterMovement))) 0.0
      (:>
        (Utilities|IsValid _returnvalue_2 :!label _label
          (:Is%20Valid
            (Pawn|SetControlRotation _returnvalue_2 (Math|Rotator|MakeRotator 0.0 0.0 0.0)))))
      (:==
        (if (Variables|Default|GetIsMovingRight?)
          (goto _label)
          (else
            (Utilities|IsValid _returnvalue :!label _label_2
              (:Is%20Valid
                (Pawn|SetControlRotation _returnvalue (Math|Rotator|MakeRotator 0.0 0.0 1.8e+02)))))))
      (:<
        (goto _label_2)))))

(event Input|ActionEvents|InputActionJump
  (params (Key :type Key%20Structure :default "None"))
  ;[1 1 1] Handle Input Events
  (:Pressed
    (if (Variables|Default|GetwallSlide?)
      (Character|LaunchCharacter (Math|Vector|MakeVector (* (.x (Transformation|GetActorForwardVector)) -1.5e+03) 0.0 6.5e+02) true true)
      (else
        (Character|Jump))))
  (:Released
    (Character|StopJumping)))

(event Input|ActionEvents|InputActionSprint
  (params (Key :type Key%20Structure :default "None"))
  ;[1 1 1] Handle Input Events
  (:Pressed
    (Variables|/Script/Engine.CharacterMovementComponent|SetMaxWalkSpeed (Variables|Character|GetCharacterMovement) (Variables|Default|GetsprintSpeed)))
  (:Released
    (Variables|/Script/Engine.CharacterMovementComponent|SetMaxWalkSpeed (Variables|Character|GetCharacterMovement) (Variables|Default|GetplayerSpeed))))

(event Input|ActionEvents|InputActionDash
  (params (Key :type Key%20Structure :default "None"))
  ;[1 1 1] Handle Input Events
  (:Pressed
    (Character|LaunchCharacter (Math|Vector|MakeVector (select (Variables|Default|GetIsMovingRight?) 3.3e+03 -3.3e+03) 0.0 0.0) true false)
    (Variables|Default|SetisDashing? true)
    (Utilities|FlowControl|RetriggerableDelay (Class|PaperFlipbook|GetTotalDuration (Variables|Animation|Getdash)))
    (Variables|Default|SetisDashing? false)))

(event Input|AxisEvents|InputAxisMoveRight
  (params (AxisValue :type Float%20%28single-precision%29))
  ;[1 1 1] Handle Input Events
  (if (> AxisValue 0.0)
    (Variables|Default|SetIsMovingRight? true)
    (elif (< AxisValue 0.0)
      (Variables|Default|SetIsMovingRight? false)))
  (Pawn|Input|AddMovementInput "1.000000, 0, 0" AxisValue false))

(fn ConstructionScript)